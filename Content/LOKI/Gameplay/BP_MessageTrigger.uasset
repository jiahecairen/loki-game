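; BP_MessageTrigger is a placeable trigger that prints a configurable message once through PrintString.
; It fires when a BP_ThirdPersonCharacter enters TriggerBox, or after a short delay on BeginPlay if ShowOnBeginPlay is set.
; Both paths share one Fired guard, so whichever comes first wins, and ShowTime optionally appends the elapsed game time in seconds.
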(event OnComponentBeginOverlap(TriggerBox)
  (params (OverlappedComponent :type Primitive%20Component%20Object%20Reference) (OtherActor :type Actor%20Object%20Reference) (OtherComp :type Primitive%20Component%20Object%20Reference) (OtherBodyIndex :type Integer) (bFromSweep :type Boolean) (SweepResult :type Hit%20Result%20Structure%20%28by%20ref%29))
  (Utilities|Casting|CastToBP_ThirdPersonCharacter OtherActor)
  (if (not (Variables|Default|GetbFired))
    (Variables|Default|SetbFired true)
    (if (Variables|Default|GetbShowTime)
      (Development|PrintString (Utilities|String|Append (Utilities|String|Append (Variables|Default|GetMessage) "  |  Time(s): ") (Utilities|String|ToString(Float) (Utilities|Time|GetTimeSeconds))) true true "(R=0.000000,G=0.660000,B=1.000000,A=1.000000)" (Variables|Default|GetDuration) "MsgTrigger")
      (else
        (Development|PrintString (Variables|Default|GetMessage) true true "(R=0.000000,G=0.660000,B=1.000000,A=1.000000)" (Variables|Default|GetDuration) "MsgTrigger")))))

(event EventBeginPlay
  (if (Variables|Default|GetbShowOnBeginPlay)
    (Utilities|FlowControl|Delay 1.0)
    (if (not (Variables|Default|GetbFired))
      (Variables|Default|SetbFired true)
      (if (Variables|Default|GetbShowTime)
        (Development|PrintString (Utilities|String|Append (Utilities|String|Append (Variables|Default|GetMessage) "  |  Time(s): ") (Utilities|String|ToString(Float) (Utilities|Time|GetTimeSeconds))) true true "(R=0.000000,G=0.660000,B=1.000000,A=1.000000)" (Variables|Default|GetDuration) "MsgTrigger")
        (else
          (Development|PrintString (Variables|Default|GetMessage) true true "(R=0.000000,G=0.660000,B=1.000000,A=1.000000)" (Variables|Default|GetDuration) "MsgTrigger"))))))

(event Collision|EventActorBeginOverlap
  (params (OtherActor :type Actor%20Object%20Reference)))

(event EventTick
  (params (DeltaSeconds :type Float%20%28single-precision%29)))

(fn ConstructionScript)