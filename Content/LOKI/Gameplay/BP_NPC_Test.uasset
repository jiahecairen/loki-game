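; BP_NPC_Test is a test NPC with placeholder dialogue that offers to open a door for the player.
; A character entering TalkBox enables input on the actor, and E toggles the conversation, locking movement while it is open.
; Keys 1 and 2 answer the pending choice, setting StoryFlagAcceptedHelp on BP_LokiGameInstance; accepting also calls OpenDoor on the BP_Door found by class.
; All prompts and lines display through PrintString.
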(event OnComponentBeginOverlap(TalkBox)
  (params (OverlappedComponent :type Primitive%20Component%20Object%20Reference) (OtherActor :type Actor%20Object%20Reference) (OtherComp :type Primitive%20Component%20Object%20Reference) (OtherBodyIndex :type Integer) (bFromSweep :type Boolean) (SweepResult :type Hit%20Result%20Structure%20%28by%20ref%29))
  (Utilities|Casting|CastToCharacter OtherActor)
  (Input|EnableInput (Game|GetPlayerController 0))
  (Development|PrintString "Press E to talk" true true "(R=0.000000,G=0.660000,B=1.000000,A=1.000000)" 3.0))

(event OnComponentEndOverlap(TalkBox)
  (params (OverlappedComponent :type Primitive%20Component%20Object%20Reference) (OtherActor :type Actor%20Object%20Reference) (OtherComp :type Primitive%20Component%20Object%20Reference) (OtherBodyIndex :type Integer))
  (Utilities|Casting|CastToCharacter OtherActor)
  (Input|DisableInput (Game|GetPlayerController 0)))

(event EventBeginPlay)

(event Collision|EventActorBeginOverlap
  (params (OtherActor :type Actor%20Object%20Reference)))

(event EventTick
  (params (DeltaSeconds :type Float%20%28single-precision%29)))

(event Input|KeyboardEvents|E
  (params (Key :type Key%20Structure))
  (:Pressed
    (if (Variables|Default|GetbTalking)
      (Variables|Default|SetbTalking false)
      (Variables|Default|SetbAwaitChoice false)
      (Input|SetIgnoreMoveInput (Game|GetPlayerController 0) false)
      (Development|PrintString " " true true "(R=0.000000,G=0.660000,B=1.000000,A=1.000000)" 0.01 "NpcDialog")
      (else
        (Variables|Default|SetbTalking true)
        (Input|SetIgnoreMoveInput (Game|GetPlayerController 0) true)
        (Variables|Default|SetbAwaitChoice true)
        (Development|PrintString "NPC：要我帮你把门打开吗？（占位对白，非正式剧情）   [1] 好   [2] 不用   [E] 关闭" true true "(R=0.000000,G=0.660000,B=1.000000,A=1.000000)" 3.6e+03 "NpcDialog")))))

(event Input|KeyboardEvents|1
  (params (Key :type Key%20Structure))
  (:Pressed
    (if (Variables|Default|GetbAwaitChoice)
      (Variables|Default|SetbAwaitChoice false)
      (bind _asbp_loki_game_instance (Utilities|Casting|CastToBP_LokiGameInstance (Game|GetGameInstance)))
      (Variables|/Game/LOKI/Gameplay/BP_LokiGameInstance.BP_LokiGameInstance_C|SetStoryFlag_AcceptedHelp _asbp_loki_game_instance true)
      (Development|PrintString "NPC：好，我来帮你开门。  [剧情标记 AcceptedHelp = true]   [E] 关闭" true true "(R=0.000000,G=0.660000,B=1.000000,A=1.000000)" 3.6e+03 "NpcDialog")
      (bind _returnvalue (Actor|GetActorOfClass "/Game/LOKI/Gameplay/BP_Door.BP_Door_C"))
      (Default|OpenDoor _returnvalue))))

(event Input|KeyboardEvents|2
  (params (Key :type Key%20Structure))
  (:Pressed
    (if (Variables|Default|GetbAwaitChoice)
      (Variables|Default|SetbAwaitChoice false)
      (bind _asbp_loki_game_instance (Utilities|Casting|CastToBP_LokiGameInstance (Game|GetGameInstance)))
      (Variables|/Game/LOKI/Gameplay/BP_LokiGameInstance.BP_LokiGameInstance_C|SetStoryFlag_AcceptedHelp _asbp_loki_game_instance false)
      (Development|PrintString "NPC：那你自己想办法吧。  [剧情标记 AcceptedHelp = false]   [E] 关闭" true true "(R=0.000000,G=0.660000,B=1.000000,A=1.000000)" 3.6e+03 "NpcDialog"))))

(fn ConstructionScript)