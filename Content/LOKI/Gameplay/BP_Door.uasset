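; BP_Door is an interactive door that rises 300 units when opened and has no logic to close again.
; Characters overlapping InteractBox enable player 0's input on the door and print an E-key prompt; leaving disables it.
; The E key and an OpenDoor event duplicate the same Open-guarded, eased MoveComponentTo on DoorMesh.
; That move feeds the actor's world location and rotation into relative-transform targets.
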(event OnComponentBeginOverlap(InteractBox)
  (params (OverlappedComponent :type Primitive%20Component%20Object%20Reference) (OtherActor :type Actor%20Object%20Reference) (OtherComp :type Primitive%20Component%20Object%20Reference) (OtherBodyIndex :type Integer) (bFromSweep :type Boolean) (SweepResult :type Hit%20Result%20Structure%20%28by%20ref%29))
  (Utilities|Casting|CastToCharacter OtherActor)
  (Input|EnableInput (Game|GetPlayerController 0))
  (Development|PrintString "Press E to open door" true true "(R=0.000000,G=0.660000,B=1.000000,A=1.000000)" 3.0))

(event OnComponentEndOverlap(InteractBox)
  (params (OverlappedComponent :type Primitive%20Component%20Object%20Reference) (OtherActor :type Actor%20Object%20Reference) (OtherComp :type Primitive%20Component%20Object%20Reference) (OtherBodyIndex :type Integer))
  (Utilities|Casting|CastToCharacter OtherActor)
  (Input|DisableInput (Game|GetPlayerController 0)))

(event Custom|OpenDoor
  (if (not (Variables|Default|GetbOpen))
    (Variables|Default|SetbOpen true)
    (Components|MoveComponentTo (Variables|Default|GetDoorMesh) (+ (Transformation|GetActorLocation) "0,0,300") (Transformation|GetActorRotation) true true 1.0 false)))

(event EventBeginPlay)

(event Collision|EventActorBeginOverlap
  (params (OtherActor :type Actor%20Object%20Reference)))

(event EventTick
  (params (DeltaSeconds :type Float%20%28single-precision%29)))

(event Input|KeyboardEvents|E
  (params (Key :type Key%20Structure))
  (:Pressed
    (if (not (Variables|Default|GetbOpen))
      (Variables|Default|SetbOpen true)
      (Components|MoveComponentTo (Variables|Default|GetDoorMesh) (+ (Transformation|GetActorLocation) "0,0,300") (Transformation|GetActorRotation) true true 1.0 false))))

(fn ConstructionScript)