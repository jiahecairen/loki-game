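; BP_Decoy is a decoy actor that lures a guard to its location.
; On BeginPlay it snaps to the nearest navmesh point, or destroys itself if projection fails.
; It then makes a one-time check on the single BP_Guard returned by GetActorOfClass, calling DecoyAttract with its location if within AttractRadius.
; Tick draws the radius and a label when the game instance's ShowDebug flag is on.
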(event EventBeginPlay
  (bind _returnvalue (Transformation|GetActorLocation))
  (bind (_projectedlocation _returnvalue_2) (AI|Navigation|ProjectPointtoNavigation _returnvalue 0 0 "800,800,500"))
  (if _returnvalue_2
    (Transformation|SetActorLocation _projectedlocation false false)
    (bind _returnvalue_3 (Actor|GetActorOfClass "/Game/LOKI/Gameplay/BP_Guard.BP_Guard_C"))
    (if (Utilities|IsValid _returnvalue_3)
      (if (< (Transformation|GetDistanceTo _returnvalue_3) (Variables|Default|GetAttractRadius))
        (Default|DecoyAttract _returnvalue_3 _returnvalue)))
    (else
      (Actor|DestroyActor))))

(event Collision|EventActorBeginOverlap
  (params (OtherActor :type Actor%20Object%20Reference)))

(event EventTick
  (params (DeltaSeconds :type Float%20%28single-precision%29))
  (bind _returnvalue (Transformation|GetActorLocation))
  (if (Variables|/Game/LOKI/Gameplay/BP_LokiGameInstance.BP_LokiGameInstance_C|GetbShowDebug (.AsBP%20Loki%20Game%20Instance (Utilities|Casting|CastToBP_LokiGameInstance (Game|GetGameInstance))))
    (Rendering|Debug|DrawDebugCircle _returnvalue (Variables|Default|GetAttractRadius) 48 "(R=1,G=0,B=1,A=1)" 0.15 1.0 "1,0,0" "0,1,0")
    (Rendering|Debug|DrawDebugString (+ _returnvalue "0,0,200") "DECOY (attracts guards in magenta radius)" 0 "(R=1,G=0,B=1,A=1)" 0.15)))

(fn ConstructionScript)