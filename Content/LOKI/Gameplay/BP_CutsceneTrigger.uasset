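; Trigger actor that plays a one-shot level sequence cutscene when the third-person character enters its box.
; On first overlap it makes the player invulnerable, enables cinematic mode, moves input from the pawn to itself and plays the sequence.
; When the sequence finishes, or Space stops it early, a shared path clears invulnerability, exits cinematic mode, blends the view back to the pawn and restores input.
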(event OnComponentBeginOverlap(TriggerBox)
  (params (OverlappedComponent :type Primitive%20Component%20Object%20Reference) (OtherActor :type Actor%20Object%20Reference) (OtherComp :type Primitive%20Component%20Object%20Reference) (OtherBodyIndex :type Integer) (bFromSweep :type Boolean) (SweepResult :type Hit%20Result%20Structure%20%28by%20ref%29))
  (bind _asbp_third_person_character (Utilities|Casting|CastToBP_ThirdPersonCharacter OtherActor))
  (if (not (Variables|Default|GetbPlayed))
    (Variables|Default|SetbPlayed true)
    (Variables|/Game/ThirdPerson/Blueprints/BP_ThirdPersonCharacter.BP_ThirdPersonCharacter_C|SetbInvulnerable _asbp_third_person_character true)
    (Class|PlayerController|SetCinematicMode (Game|GetPlayerController 0) true true true true true)
    (bind _returnvalue (Sequencer|Player|CreateLevelSequencePlayer (Variables|Default|GetSequence)))
    (Variables|Default|SetSeqPlayer _returnvalue)
    (Variables|Default|SetbPlaying true)
    (EventDispatchers|BindEventtoOnFinished _returnvalue (delegate Custom|SequenceFinished))
    (Sequencer|Player|Play _returnvalue :!class /Script/MovieScene.MovieSceneSequencePlayer)
    (Input|EnableInput (Game|GetPlayerController 0))
    (Input|DisableInput (Game|Player|GetPlayerPawn 0) (Game|GetPlayerController 0))
    (Development|PrintString "Press SPACE to skip" true true "(R=0.000000,G=0.660000,B=1.000000,A=1.000000)" 5.0 "CutsceneSkip")))

(event Custom|SequenceFinished
  (Variables|Default|SetbPlaying false)
  (Variables|/Game/ThirdPerson/Blueprints/BP_ThirdPersonCharacter.BP_ThirdPersonCharacter_C|SetbInvulnerable (.AsBP%20Third%20Person%20Character (Utilities|Casting|CastToBP_ThirdPersonCharacter (Game|Player|GetPlayerPawn 0))) false)
  (Class|PlayerController|SetCinematicMode (Game|GetPlayerController 0) false true true true true)
  (Game|Player|SetViewTargetwithBlend (Game|GetPlayerController 0) (Game|Player|GetPlayerPawn 0) 0.3 "VTBlend_Linear" 0.0 false)
  (Input|DisableInput (Game|GetPlayerController 0))
  (Input|EnableInput (Game|Player|GetPlayerPawn 0) (Game|GetPlayerController 0)))

(event EventBeginPlay)

(event Collision|EventActorBeginOverlap
  (params (OtherActor :type Actor%20Object%20Reference)))

(event EventTick
  (params (DeltaSeconds :type Float%20%28single-precision%29)))

(event Input|KeyboardEvents|SpaceBar
  (params (Key :type Key%20Structure))
  (:Pressed
    (if (Variables|Default|GetbPlaying)
      (Sequencer|Player|Stop (Variables|Default|GetSeqPlayer) :!class /Script/MovieScene.MovieSceneSequencePlayer)
      (Variables|Default|SetbPlaying false)
      (Variables|/Game/ThirdPerson/Blueprints/BP_ThirdPersonCharacter.BP_ThirdPersonCharacter_C|SetbInvulnerable (.AsBP%20Third%20Person%20Character (Utilities|Casting|CastToBP_ThirdPersonCharacter (Game|Player|GetPlayerPawn 0))) false)
      (Class|PlayerController|SetCinematicMode (Game|GetPlayerController 0) false true true true true)
      (Game|Player|SetViewTargetwithBlend (Game|GetPlayerController 0) (Game|Player|GetPlayerPawn 0) 0.3 "VTBlend_Linear" 0.0 false)
      (Input|DisableInput (Game|GetPlayerController 0))
      (Input|EnableInput (Game|Player|GetPlayerPawn 0) (Game|GetPlayerController 0)))))

(fn ConstructionScript)