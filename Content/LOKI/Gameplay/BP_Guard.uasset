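; BP_Guard is a knight enemy that patrols between two points, chases and attacks the player, and can be lured away by decoys.
; Pawn sensing, a proximity line-of-sight check and taking damage trigger a chase, which ends when the target goes unseen too long or the player cloaks.
; Self-rescheduling Delay loops drive patrol, detection, chase, debug drawing and single-node animation switching.
; Damage flashes the mesh material, and death plays an animation before destroying the actor.
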(event OnSeePawn(PawnSensing)
  (params (Pawn :type Pawn%20Object%20Reference))
  (Variables|Default|SetTargetPawn Pawn)
  (Variables|Default|SetLastSeenTime (Utilities|Time|GetGameTimeinSeconds))
  (if (not (or (or (Variables|Default|GetbChasing) (Variables|Default|GetbDistracted)) (Variables|/Game/ThirdPerson/Blueprints/BP_ThirdPersonCharacter.BP_ThirdPersonCharacter_C|GetbCloaked (.AsBP%20Third%20Person%20Character (Utilities|Casting|CastToBP_ThirdPersonCharacter (Game|Player|GetPlayerPawn 0))))))
    (Variables|Default|SetbChasing true)
    (Development|SetHiddeninGame (Variables|Default|GetAlertMark) false false)
    (Variables|/Script/Engine.CharacterMovementComponent|SetMaxWalkSpeed (Variables|Character|GetCharacterMovement) 3e+02)
    (Development|PrintString "Guard: Alert! (chasing player)" true true "(R=0.000000,G=0.660000,B=1.000000,A=1.000000)" 3.0 "GuardState")
    (bind _asai控制器 (Utilities|Casting|CastToAIController (Pawn|GetController)))
    (AI|Navigation|MovetoActor _asai控制器 Pawn 1e+02 true true true 0)
    (CallFunction|ChaseLoop)))

(event Custom|Patrol
  (if (or (Variables|Default|GetbChasing) (Variables|Default|GetbDistracted))
    (Utilities|FlowControl|Delay 1.0)
    (else
      (bind _asai控制器 (Utilities|Casting|CastToAIController (Pawn|GetController)))
      (if (Variables|Default|GetbGoToB)
        (AI|Navigation|MovetoLocation _asai控制器 (Variables|Default|GetPointB) 5e+01 true true false true 0)
        (else
          (AI|Navigation|MovetoLocation _asai控制器 (Variables|Default|GetPointA) 5e+01 true true false true 0)))
      (Variables|Default|SetbGoToB (not (Variables|Default|GetbGoToB)))
      (Utilities|FlowControl|Delay 5.0)))
  (CallFunction|Patrol))

(event Custom|ChaseLoop
  (if (Variables|Default|GetbChasing)
    (bind _asai控制器 (Utilities|Casting|CastToAIController (Pawn|GetController)))
    (AI|Navigation|MovetoActor _asai控制器 (Variables|Default|GetTargetPawn) 25.0 true true true 0)
    (if (and (and (< (Transformation|GetDistanceTo (Variables|Default|GetTargetPawn)) 1.6e+02) (not (Variables|Default|GetbAtkCD))) (not (Variables|Default|GetbDead)))
      (CallFunction|GuardAttack))
    (if (or (> (- (Utilities|Time|GetGameTimeinSeconds) (Variables|Default|GetLastSeenTime)) (Variables|Default|GetLoseTargetSeconds)) (Variables|/Game/ThirdPerson/Blueprints/BP_ThirdPersonCharacter.BP_ThirdPersonCharacter_C|GetbCloaked (.AsBP%20Third%20Person%20Character (Utilities|Casting|CastToBP_ThirdPersonCharacter (Game|Player|GetPlayerPawn 0)))))
      (AI|Navigation|StopMovement _asai控制器)
      (Variables|Default|SetbChasing false)
      (Development|SetHiddeninGame (Variables|Default|GetAlertMark) true false)
      (Variables|/Script/Engine.CharacterMovementComponent|SetMaxWalkSpeed (Variables|Character|GetCharacterMovement) 1.2e+02)
      (Development|PrintString "Guard: lost target, back to patrol" true true "(R=0.000000,G=0.660000,B=1.000000,A=1.000000)" 3.0 "GuardState")
      (else
        (Utilities|FlowControl|Delay 0.15)
        (CallFunction|ChaseLoop)))))

(event Custom|ProximityLoop
  (if (< (Transformation|GetDistanceTo (Game|Player|GetPlayerPawn 0)) (Variables|Default|GetProximityRadius))
    (if (Variables|Default|GetbChasing)
      _
      (else
        (bind _asai控制器 (Utilities|Casting|CastToAIController (Pawn|GetController))
          (:then
            (if (Controller|LineOfSightTo _asai控制器 (Game|Player|GetPlayerPawn 0) "0, 0, 0" false)
              (CallFunction|SpotPlayer)))
          (:CastFailed
            _)))))
  (Utilities|FlowControl|Delay 0.2)
  (CallFunction|ProximityLoop))

(event Custom|SpotPlayer
  (Variables|Default|SetTargetPawn (Game|Player|GetPlayerPawn 0))
  (Variables|Default|SetLastSeenTime (Utilities|Time|GetGameTimeinSeconds))
  (if (not (or (or (Variables|Default|GetbChasing) (Variables|Default|GetbDistracted)) (Variables|/Game/ThirdPerson/Blueprints/BP_ThirdPersonCharacter.BP_ThirdPersonCharacter_C|GetbCloaked (.AsBP%20Third%20Person%20Character (Utilities|Casting|CastToBP_ThirdPersonCharacter (Game|Player|GetPlayerPawn 0))))))
    (Variables|Default|SetbChasing true)
    (Development|SetHiddeninGame (Variables|Default|GetAlertMark) false false)
    (Variables|/Script/Engine.CharacterMovementComponent|SetMaxWalkSpeed (Variables|Character|GetCharacterMovement) 3e+02)
    (Development|PrintString "Guard: Alert! (chasing player)" true true "(R=0.000000,G=0.660000,B=1.000000,A=1.000000)" 3.0 "GuardState")
    (bind _asai控制器 (Utilities|Casting|CastToAIController (Pawn|GetController)))
    (AI|Navigation|MovetoActor _asai控制器 (stale OnSeePawn(PawnSensing) Pawn) 1e+02 true true true 0)
    (CallFunction|ChaseLoop)))

(event Custom|DecoyAttract
  (params (Where :type Vector))
  (Variables|Default|SetbChasing false)
  (Development|SetHiddeninGame (Variables|Default|GetAlertMark) true false)
  (Variables|Default|SetbDistracted true)
  (Variables|/Script/Engine.CharacterMovementComponent|SetMaxWalkSpeed (Variables|Character|GetCharacterMovement) 2e+02)
  (bind _asai控制器 (Utilities|Casting|CastToAIController (Pawn|GetController)))
  (AI|Navigation|StopMovement _asai控制器)
  (AI|Navigation|MovetoLocation _asai控制器 Where 5e+01 true true false true 0)
  (Development|PrintString "Guard: distracted by decoy" true true "(R=0.000000,G=0.660000,B=1.000000,A=1.000000)" 3.0 "GuardState")
  (Utilities|FlowControl|Delay 4.0)
  (Variables|Default|SetbDistracted false)
  (if (not (Variables|Default|GetbChasing))
    (Variables|/Script/Engine.CharacterMovementComponent|SetMaxWalkSpeed (Variables|Character|GetCharacterMovement) 1.2e+02)))

(event Custom|GuardAttack
  (if (not (Class|LokiHealthComponent|IsActorDead (Variables|Default|GetTargetPawn)))
    (Variables|Default|SetbAtkCD true)
    (Variables|Default|SetbAttackAnim true)
    (Components|Animation|PlayAnimation (Variables|Character|GetMesh) "/Game/LastWizard/Characters/Knight/Animations/A_Knight_Attack.A_Knight_Attack" false)
    (Components|Timeline|SetPlayRate (Variables|Character|GetMesh) 2.0)
    (Game|Damage|ApplyDamage (Variables|Default|GetTargetPawn) (Variables|Default|GetGuardDamage) (Pawn|GetController) self)
    (Development|PrintString "Guard attacks!" true true "(R=0.000000,G=0.660000,B=1.000000,A=1.000000)" 1.0 "GuardAtk")
    (Utilities|FlowControl|Delay 1.0)
    (Variables|Default|SetbAtkCD false)
    (Variables|Default|SetbAttackAnim false)
    (Variables|Default|SetCurAnim 0)
    (Components|Timeline|SetPlayRate (Variables|Character|GetMesh) 1.0)))

(event Custom|DebugLoop
  (bind _returnvalue (Transformation|GetActorLocation))
  (bind _returnvalue_2 (+ _returnvalue "0,0,170"))
  (if (Variables|/Game/LOKI/Gameplay/BP_LokiGameInstance.BP_LokiGameInstance_C|GetbShowDebug (.AsBP%20Loki%20Game%20Instance (Utilities|Casting|CastToBP_LokiGameInstance (Game|GetGameInstance))))
    (Class|KismetSystemLibrary|DrawDebugConeinDegrees (+ _returnvalue "0,0,-80") (Transformation|GetActorForwardVector) (Variables|/Script/AIModule.PawnSensingComponent|GetSightRadius (Variables|Default|GetPawnSensing)) 9e+01 1.0 16 "(R=1,G=1,B=0,A=1)" 0.15 1.0 "World")
    (if (Variables|Default|GetbChasing)
      (Rendering|Debug|DrawDebugString _returnvalue_2 "CHASE" 0 "(R=1,G=0,B=0,A=1)" 0.15)
      (elif (Variables|Default|GetbDistracted)
        (Rendering|Debug|DrawDebugString _returnvalue_2 "DISTRACTED" 0 "(R=0.3,G=0.5,B=1,A=1)" 0.15)
        (else
          (Rendering|Debug|DrawDebugString _returnvalue_2 "PATROL" 0 "(R=0,G=1,B=0,A=1)" 0.15)))))
  (Utilities|FlowControl|Delay 0.05)
  (CallFunction|DebugLoop))

(event Custom|AnimLoop
  (bind _returnvalue (Transformation|GetVelocity))
  (bind _returnvalue_2 (Math|Vector|VectorLength _returnvalue))
  (if (not (Variables|Default|GetbDead))
    (if (Variables|Default|GetbAttackAnim)
      _
      (elif (> _returnvalue_2 2e+01)
        (Components|Timeline|SetPlayRate (Variables|Character|GetMesh) (/ _returnvalue_2 (Variables|Default|GetWalkRefSpeed)))
        (if (!= (Variables|Default|GetCurAnim) 2)
          (Variables|Default|SetCurAnim 2)
          (Components|Animation|PlayAnimation (Variables|Character|GetMesh) "/Game/LastWizard/Characters/Knight/Animations/A_Knight_Walk.A_Knight_Walk" true))
        (elif (!= (Variables|Default|GetCurAnim) 1)
          (Variables|Default|SetCurAnim 1)
          (Components|Animation|PlayAnimation (Variables|Character|GetMesh) "/Game/LastWizard/Characters/Knight/Animations/A_Knight_Idle.A_Knight_Idle" true))))
    (Utilities|FlowControl|Delay 0.1)
    (CallFunction|AnimLoop)))

(event EventBeginPlay
  (Variables|Default|SetPointA (Transformation|GetActorLocation))
  (Variables|Default|SetPointB (+ (Variables|Default|GetPointA) (Variables|Default|GetPatrolOffset)))
  (Utilities|FlowControl|Sequence
    (:then_0
      (CallFunction|Patrol))
    (:then_1
      (CallFunction|ProximityLoop))
    (:then_2
      (CallFunction|DebugLoop))
    (:then_3
      (CallFunction|AnimLoop))))

(event Collision|EventActorBeginOverlap
  (params (OtherActor :type Actor%20Object%20Reference)))

(event EventTick
  (params (DeltaSeconds :type Float%20%28single-precision%29)))

(event Game|Damage|EventAnyDamage
  (params (Damage :type Float%20%28single-precision%29) (DamageType :type Damage%20Type%20Object%20Reference) (InstigatedBy :type Controller%20Object%20Reference) (DamageCauser :type Actor%20Object%20Reference))
  (bind _mesh (Variables|Character|GetMesh))
  (bind _mesh_2 (Variables|Character|GetMesh))
  (if (not (Variables|Default|GetbDead))
    (bind _output_get (Variables|Default|SetHealth (- (Variables|Default|GetHealth) Damage)))
    (Development|PrintString (Utilities|String|ToString(Float) _output_get) true true "(R=0.000000,G=0.660000,B=1.000000,A=1.000000)" 2.0 "GuardHP")
    (Utilities|FlowControl|Sequence
      (:then_0
        (Rendering|Material|SetMaterial _mesh 0 "/Game/LOKI/Materials/M_Ghost.M_Ghost")
        (Rendering|Material|SetMaterial _mesh 1 "/Game/LOKI/Materials/M_Ghost.M_Ghost")
        (Utilities|FlowControl|Delay 0.15)
        (Rendering|Material|SetMaterial _mesh 0 "/Game/LastWizard/Characters/Knight/Materials/MI_Knight_Top.MI_Knight_Top")
        (Rendering|Material|SetMaterial _mesh 1 "/Game/LastWizard/Characters/Knight/Materials/MI_Knight.MI_Knight"))
      (:then_1
        (if (<= _output_get 0.0)
          (Variables|Default|SetbDead true)
          (Development|SetHiddeninGame (Variables|Default|GetAlertMark) true false)
          (bind _asai控制器 (Utilities|Casting|CastToAIController (Pawn|GetController)))
          (AI|Navigation|StopMovement _asai控制器)
          (Pawn|Components|CharacterMovement|DisableMovement (Variables|Character|GetCharacterMovement))
          (Collision|SetCollisionEnabled (Variables|Collision|GetCapsuleComponent) "NoCollision")
          (Collision|SetCollisionProfileName _mesh_2 "Ragdoll" true :!class /Script/Engine.PrimitiveComponent)
          (Physics|SetSimulatePhysics _mesh_2 false)
          (Components|Animation|PlayAnimation (Variables|Character|GetMesh) "/Game/LastWizard/Characters/Knight/Animations/A_Knight_Death.A_Knight_Death" false)
          (Development|PrintString "Guard: defeated" true true "(R=0.000000,G=0.660000,B=1.000000,A=1.000000)" 3.0 "GuardHP")
          (Utilities|FlowControl|Delay 5.0)
          (Actor|DestroyActor)
          (else
            (CallFunction|SpotPlayer)))))))

(fn ConstructionScript)